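; BP_Lever is an interactable lever prop that signals a linked gate, with an optional single-use setting.
; Interact plays a pull sound and alternates between two timelines that roll the handle, ignoring input while animating.
; A delay started from timeline updates clears the animation lock and sends OpenGateMessage to LinkedGate on pulls in either direction.
; An overlap sphere toggles a widget's visibility for the player character's class.
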(event `/Game/CustomContent/GameFramework/BI_Interaction.Interact`
  (if (not (`self.animating`))
    (if (`self.singleUse`)
      (`/Engine/EditorBlueprintResources/StandardMacros.DoOnce` false
        (:`Completed`
          _)))
    (set `self.animating` true)
    (`GameplayStatics.PlaySoundAtLocation` (`self.leverPullSound`) (`self.K2_GetActorLocation`) (struct) 1.0 1.0 0.0 null null null null)
    (if (`self.pulled`)
      (set `self.pulled` false)
      (bind (_direction _opentrack) (`Timeline|Timeline_0` :!via `PlayFromStart`)
        (:`Update`
          (`SceneComponent.K2_SetRelativeRotation` (`self.Handle`) (`KismetMathLibrary.MakeRotator` _opentrack) false false)))
      (else
        (set `self.pulled` true)
        (bind (_direction_2 _opentrack_2) (`Timeline|Timeline` :!via `PlayFromStart`)
          (:`Update`
            (`SceneComponent.K2_SetRelativeRotation` (`self.Handle`) (`KismetMathLibrary.MakeRotator` _opentrack_2) false false)))))
    (`KismetSystemLibrary.Delay` 0.6)
    (set `self.animating` false)
    (message `/Game/CustomContent/GameFramework/BI_Interaction.openGate` (`self.linkedGate`))))

(event `self.Sphere.OnComponentBeginOverlap`
  (params (OverlappedComponent :type "PrimitiveComponent Object Reference") (OtherActor :type "Actor Object Reference") (OtherComp :type "PrimitiveComponent Object Reference") (OtherBodyIndex :type Integer) (bFromSweep :type Boolean) (SweepResult :type "HitResult Structure (by ref)"))
  (if (== (`GameplayStatics.GetObjectClass` OtherActor) (`GameplayStatics.GetObjectClass` (`GameplayStatics.GetPlayerCharacter` 0)))
    (`SceneComponent.SetVisibility` (`self.Widget`) true false)))

(event `self.Sphere.OnComponentEndOverlap`
  (params (OverlappedComponent :type "PrimitiveComponent Object Reference") (OtherActor :type "Actor Object Reference") (OtherComp :type "PrimitiveComponent Object Reference") (OtherBodyIndex :type Integer))
  (if (== (`GameplayStatics.GetObjectClass` OtherActor) (`GameplayStatics.GetObjectClass` (`GameplayStatics.GetPlayerCharacter` 0)))
    (`SceneComponent.SetVisibility` (`self.Widget`) false false)))

(fn `getIsGamepad`
  (returns (isGamepad :type Boolean))
  (return false))

(fn `removeKey`
  (returns (Success :type Boolean))
  (return false))

(fn `UserConstructionScript`)