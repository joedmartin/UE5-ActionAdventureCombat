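; BP_PatrolRoute defines a spline-based patrol path for enemy AI.
; IncrementPatrol steps PatrolIndex along the spline points, flipping Direction at the last and first points for back-and-forth movement.
; GetSplinePointAsWorldPosition returns the current point's location in world space.
; The blocking, sprinting, patrol route, melee animation and ranged strength getters are stubs returning default or empty values.
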(event `/Game/CustomContent/GameFramework/BI_CharacterActions.incrementPatrol`
  (bind _output_get (set `self.patrolIndex` (+ (`self.patrolIndex`) (`self.direction`))))
  (if (== _output_get (- (`SplineComponent.GetNumberOfSplinePoints` (`self.PatrolRoute`)) 1))
    (set `self.direction` -1)
    (elif (== (`self.patrolIndex`) 0)
      (set `self.direction` 1))))

(fn `getIsBlocking`
  (returns (isBlocking :type Boolean))
  (return false))

(fn `getIsSprinting`
  (returns (isSprinting :type Boolean))
  (return false))

(fn `getPatrolRoute`
  (returns (patrolRoute :type "/Game/CustomContent/Enemies/AI/BP_PatrolRoute Object Reference"))
  (return null))

(fn `getRandomMeleeAnim`
  (returns (meleeAnims :type "AnimMontage Object Reference"))
  (return null))

(fn `getRangedStrength`
  (returns (rangedStrength :type "Float (double-precision)"))
  (return 0.0))

(fn `GetSplinePointAsWorldPosition`
  (returns (Location :type "Vector Structure"))
  (return (`SplineComponent.GetLocationAtSplinePoint` (`self.PatrolRoute`) (`self.patrolIndex`) "World")))

(fn `UserConstructionScript`)