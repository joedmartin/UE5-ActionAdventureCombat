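; Ice projectile actor for enemy ranged attacks that damages what it overlaps and bursts on contact.
; Sphere overlap applies damage using the ranged strength queried from the instigator.
; Both hit and overlap swap the particle template to an explosion, stop movement and destroy the actor after a short delay.
; The enemy-related getter and attack-token functions are stubs returning empty or default values.
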(event `self.Sphere.OnComponentHit`
  (params (HitComponent :type "PrimitiveComponent Object Reference") (OtherActor :type "Actor Object Reference") (OtherComp :type "PrimitiveComponent Object Reference") (NormalImpulse :type "Vector Structure") (Hit :type "HitResult Structure (by ref)"))
  (`ParticleSystemComponent.SetTemplate` (`self.ParticleSystem`) (`self.explosionParticleTemplate`) :!label _label)
  (`MovementComponent.StopMovementImmediately` (`self.ProjectileMovement`))
  (`KismetSystemLibrary.Delay` 0.5)
  (`self.K2_DestroyActor`))

(event `self.Sphere.OnComponentBeginOverlap`
  (params (OverlappedComponent :type "PrimitiveComponent Object Reference") (OtherActor :type "Actor Object Reference") (OtherComp :type "PrimitiveComponent Object Reference") (OtherBodyIndex :type Integer) (bFromSweep :type Boolean) (SweepResult :type "HitResult Structure (by ref)"))
  (bind _rangedstrength (message `/Game/CustomContent/GameFramework/BI_CharacterActions.getRangedStrength` (`self.GetInstigator`)))
  (`GameplayStatics.ApplyDamage` OtherActor _rangedstrength)
  (goto _label))

(fn `getIsBlocking`
  (returns (isBlocking :type Boolean))
  (return false))

(fn `getIsSprinting`
  (returns (isSprinting :type Boolean))
  (return false))

(fn `getPatrolRoute`
  (returns (patrolRoute :type "/Game/CustomContent/Enemies/AI/BP_PatrolRoute Object Reference"))
  (return null))

(fn `getRandomMeleeAnim`
  (returns (meleeAnims :type "AnimMontage Object Reference"))
  (return null))

(fn `getRangedStrength`
  (returns (rangedStrength :type "Float (double-precision)"))
  (return 0.0))

(fn `reserveAttackToken`
  (params (Amount :type Integer))
  (returns (Success :type Boolean))
  (return false))

(fn `UserConstructionScript`)